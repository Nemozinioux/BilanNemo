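; BP_QuestSolution is an interactable quest target that completes a step of a quest when the player carries the quest item.
; On Interact, it checks the quest-item flag on GI_MainInstance and its own IsObjective flag.
; If both are set, it swaps the cube's material and calls ValidateStep on the player character's ACQuestManager with a hardcoded quest and step.
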(event `/Game/InteractionSystem/BPI_Interactible.Interact`
  (bind _asgi_main_instance (cast `/Game/GI_MainInstance` (`GameplayStatics.GetGameInstance`)))
  (if (and (`/Game/GI_MainInstance.PlayerHasQuestItem` _asgi_main_instance) (`self.IsObjective`))
    (`PrimitiveComponent.SetMaterial` (`self.Cube`) 0 "/Engine/MapTemplates/Materials/BasicAsset03.BasicAsset03")
    (bind _asbp_first_person_character (cast `/Game/FirstPerson/Blueprints/BP_FirstPersonCharacter` (`GameplayStatics.GetPlayerCharacter` 0)))
    (`/Game/QuestSystem/AC_QuestManager.ValidateStep` (`/Game/FirstPerson/Blueprints/BP_FirstPersonCharacter.AC_QuestManager` _asbp_first_person_character) "Quest1" 1)))

(fn `UserConstructionScript`)